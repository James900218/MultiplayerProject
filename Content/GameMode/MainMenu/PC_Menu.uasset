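; PC_Menu is the player controller for the main menu, responsible for putting the menu UI on screen.
; On BeginPlay, for the local controller only, it creates the W_MainMenu widget for player controller 0 and adds it to the viewport.
; It then shows the mouse cursor and switches input to Game and UI mode, focused on that widget.
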(event EventBeginPlay
  (if (Pawn|IsLocalPlayerController)
    (bind _output_get (Variables|Default|SetPC_Menu (Game|GetPlayerController 0)))
    (bind _returnvalue (UserInterface|CreateWidget "/Game/GameMode/MainMenu/W_MainMenu.W_MainMenu_C" _output_get))
    (bind _output_get_2 (Variables|Default|SetMenu_UI _returnvalue))
    (UserInterface|Viewport|AddtoViewport _output_get_2 0)
    (Variables|Default|SetbShowMouseCursor true)
    (Input|SetInputModeGameandUI (Variables|Default|GetPC_Menu) (Variables|Default|GetMenu_UI) "DoNotLock" true false)))

(fn ConstructionScript)