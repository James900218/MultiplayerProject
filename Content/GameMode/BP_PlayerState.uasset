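; Player state for the TPS game that tracks a player's score and reports it to BP_TPSGameState.
; The construction script binds OnPawnSet, whose handler marks PawnReady once a valid pawn is assigned.
; AddToPlayerScore increments the score, then passes it to the game state's REPUpdatePlayerScore.
; That update, also attempted on BeginPlay, only runs when PawnReady is true.
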(event Custom|AddScoreToGameState
  (bind _asbp_tpsgame_state (Utilities|Casting|CastToBP_TPSGameState (Game|GetGameState))
    (:then
      (if (Variables|Default|GetPawnReady)
        (Default|REPUpdatePlayerScore _asbp_tpsgame_state self (Variables|Default|GetPlayerScore))))
    (:CastFailed
      (Development|PrintString "CAST FAILED (BP_TPSGameState) in BP_PlayerState"))))

(event Custom|AddToPlayerScore
  (params (AddToScore :type Integer))
  (Variables|Default|SetPlayerScore (+ (Variables|Default|GetPlayerScore) AddToScore))
  (CallFunction|AddScoretoGameState))

(event EventBeginPlay
  (bind _asbp_tpsgame_state (Utilities|Casting|CastToBP_TPSGameState (Game|GetGameState)))
  (if (Variables|Default|GetPawnReady)
    (Default|REPUpdatePlayerScore _asbp_tpsgame_state self (Variables|Default|GetPlayerScore))))

(event EventTick
  (params (DeltaSeconds :type Float%20%28single-precision%29)))

(fn ConstructionScript
  (Events|BindEventtoOnPawnSet (EventDispatchers|CreateEvent :!event BPPlayerStateAutoGenFunc)))

(fn BPPlayerStateAutoGenFunc
  (params (Player :type Player%20State%20Object%20Reference) (NewPawn :type Pawn%20Object%20Reference) (OldPawn :type Pawn%20Object%20Reference))
  (Utilities|IsValid NewPawn
    (:Is%20Valid
      (Variables|Default|SetPawnReady true))))