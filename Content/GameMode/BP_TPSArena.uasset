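; BP_TPSArena is a third-person shooter arena game mode that respawns players at random spawn points.
; On BeginPlay it caches every BP_SpawnPoint actor in the level.
; RespawnPlayer takes a random cached point's transform via LookForSpawnPoints, spawns a new actor of the passed player's class there, has the given controller possess it and prints a debug message.
; It neither checks whether the point is occupied nor destroys the old pawn.
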(event Custom|RespawnPlayer
  (params (Player :type Character%20Object%20Reference) (PController :type Controller%20Object%20Reference))
  (CallFunction|LookforSpawnPoints)
  (bind _returnvalue (Game|SpawnActorfromClass (Utilities|GetClass Player) (Variables|Default|GetSpawnTransform) "Undefined" "MultiplyWithRoot" 0 0))
  (Pawn|Possess PController _returnvalue)
  (Development|PrintString "RESPAWNING"))

(event Custom|LookForSpawnPoints
  (Variables|Default|SetSpawnTransform (Transformation|GetActorTransform (.OutItem (Utilities|Array|Random (Variables|Default|GetSpawn%20Points))))))

(event EventBeginPlay
  (bind _outactors (Actor|GetAllActorsOfClass "/Game/_Main/SpawnPoints/BP_SpawnPoint.BP_SpawnPoint_C"))
  (Variables|Default|SetSpawn%20Points _outactors))

(event EventTick
  (params (DeltaSeconds :type Float%20%28single-precision%29)))

(fn ConstructionScript)