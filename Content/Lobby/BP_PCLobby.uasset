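; Lobby player controller that shows the lobby UI and reports the player's ready state and character choice to BP_LobbyGM.
; On BeginPlay the local controller creates W_LobbyUI, enables the mouse and requests a server-side info update.
; Server events toggle PlayerInfo.Ready or set SelectedCharacterClass, whose RepNotify calls the game mode's UpdatePlayerInfo, effective only on the server.
; A separate UpdatePlayerInfo event resends after a short delay.
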(event Custom|UpdatePlayerInfo
  (Utilities|FlowControl|Delay 0.1)
  (CallFunction|RunonServerUpdatePlayerInfo))

(event Custom|RunOnServer_UpdatePlayerInfo
  (bind _asbp_lobby_gm (Utilities|Casting|CastToBP_LobbyGM (Game|GetGameMode)))
  (Default|UpdatePlayerInfo _asbp_lobby_gm self))

(event Custom|ROS_ToggleReadyStatus
  (bind _playerinfo (Variables|Default|GetPlayerInfo))
  (Utilities|Struct|SetmembersinS_PlayerInfo _playerinfo (not (.Ready (Utilities|Struct|BreakS_PlayerInfo _playerinfo))))
  (bind _asbp_lobby_gm (Utilities|Casting|CastToBP_LobbyGM (Game|GetGameMode)))
  (Default|UpdatePlayerInfo _asbp_lobby_gm self))

(event Custom|ROS_UpdateSelectedCharacter
  (params (SelectedCharacterClass :type BP%20Third%20Person%20Character%20Class%20Reference))
  (Variables|Default|SetSelectedCharacterClass SelectedCharacterClass))

(event EventBeginPlay
  (if (Pawn|IsLocalPlayerController)
    (bind _returnvalue (UserInterface|CreateWidget "/Game/_Main/Hud/W_LobbyUI.W_LobbyUI_C"))
    (bind _output_get (Variables|Default|SetLobbyUI _returnvalue))
    (UserInterface|Viewport|AddtoViewport _output_get 0)
    (Variables|Default|SetbShowMouseCursor true)
    (Input|SetInputModeGameandUI self (Variables|Default|GetLobbyUI) "DoNotLock" true false)
    (CallFunction|RunonServerUpdatePlayerInfo)))

(fn ConstructionScript)

(fn OnRepSelectedCharacterClass
  (bind _asbp_lobby_gm (Utilities|Casting|CastToBP_LobbyGM (Game|GetGameMode)))
  (Default|UpdatePlayerInfo _asbp_lobby_gm self))