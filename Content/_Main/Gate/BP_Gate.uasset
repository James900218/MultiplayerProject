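; BP_Gate is a gate actor that can be progressively damaged, repaired and finally knocked down.
; DestroyGate raises GateAngle and adds it to the actor's roll with a bang, while RepairGate lowers it and tilts back with a clang.
; Once GateAngle reaches its limit, a timeline rolls the gate flat, replaying a falling sound on each update and disabling mesh and box collision after a short delay.
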(event EventBeginPlay)

(event Collision|EventActorBeginOverlap
  (params (OtherActor :type Actor%20Object%20Reference)))

(event EventTick
  (params (DeltaSeconds :type Float%20%28single-precision%29)))

(event EventDestroyGate
  (bind _returnvalue (Transformation|GetActorRotation))
  (bind _returnvalue_2 (Transformation|GetActorRotation))
  (bind _collbox (Variables|Default|GetCollBox))
  (bind _returnvalue_3 (Transformation|GetWorldLocation _collbox))
  (if (< (Variables|Default|GetGateAngle) 2.0)
    (bind _output_get (Variables|Default|SetGateAngle (+ (Variables|Default|GetGateAngle) 0.1)))
    (Transformation|SetActorRotation (Math|Rotator|MakeRotator (+ _output_get (.roll _returnvalue)) (.pitch _returnvalue) (.yaw _returnvalue)))
    (Audio|PlaySoundatLocation "/Game/Interface_And_Item_Sounds/MoreSounds/MetalBang.MetalBang" _returnvalue_3 "0, 0, 0" 1.0 0.25 0.0 0 0 0 0)
    (else
      (Utilities|FlowControl|Sequence
        (:then_0
          (bind _newtrack_0 (Timeline|GateFallingTL Play)
            (:Update
              (Audio|PlaySoundatLocation "/Game/Interface_And_Item_Sounds/MoreSounds/MetalFalling.MetalFalling" _returnvalue_3 "0, 0, 0" 0.5 1.0 0.0 0 0 0 0)
              (Transformation|SetActorRotation (Math|Rotator|MakeRotator (Math|Float|MapRangeClamped _newtrack_0 0.0 9e+01 (.roll _returnvalue_2) 9e+01) (.pitch _returnvalue_2) (.yaw _returnvalue_2)))
              (Utilities|FlowControl|Delay 0.5)
              (Collision|SetCollisionEnabled (Variables|Default|GetGate%20Mesh1) "NoCollision")
              (Collision|SetCollisionEnabled (Variables|Default|GetCollBox) "NoCollision")
              (Collision|SetCollisionEnabled (Variables|Default|GetGate%20Mesh) "NoCollision"))))))))

(event EventRepairGate
  (bind _returnvalue (Transformation|GetActorRotation))
  (bind _output_get (Variables|Default|SetGateAngle (- (Variables|Default|GetGateAngle) 0.1)))
  (Transformation|SetActorRotation (Math|Rotator|MakeRotator (- (.roll _returnvalue) _output_get) (.pitch _returnvalue) (.yaw _returnvalue)))
  (Audio|PlaySoundatLocation "/Game/Interface_And_Item_Sounds/MoreSounds/MetalClang.MetalClang" (Transformation|GetWorldLocation (Variables|Default|GetCollBox)) "0, 0, 0" 1.0 1.0 0.0 0 0 0 0))

(fn ConstructionScript)